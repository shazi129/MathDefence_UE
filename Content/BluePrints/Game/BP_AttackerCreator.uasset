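; Spawner actor for BP_Attacker, which CreateAttacker places at reduced scale at a random X offset within half the Left-to-Right marker span around the actor.
; It registers as a listener on the singleton MDGameNotifier; its start-check-result handler only prints the input result's number.
; CreateAttacker is not called within this Blueprint, and IsMainGameNotify leaves its notifier comparison unconnected.
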(event EventBeginPlay
  (bind _self self)
  (CallFunction|Init)
  (Class|GameNotifier|AddListener (Variables|Default|GetMainGameNotifier) _self)
  (Development|PrintString (Utilities|GetDisplayName _self)))

(event Collision|EventActorBeginOverlap
  (params (OtherActor :type Actor%20Object%20Reference)))

(event EventTick
  (params (DeltaSeconds :type Float%20%28single-precision%29)))

(event EventUpdateSelf
  (params (notifyData :type Game%20Notify%20Data%20Structure%20%28by%20ref%29))
  (if (Utilities|IsMainGameNotify notifyData)
    (CallFunction|HandleMainGameNotify notifyData)))

(event EventDestroyed
  (Class|GameNotifier|RemoveListener (Variables|Default|GetMainGameNotifier) self))

(fn ConstructionScript)

(fn PrintTime
  (bind _returnvalue (Class|MyTimeUtils|Now))
  (Development|PrintString (Utilities|String|ToString(Integer) _returnvalue)))

(fn RandomPosition
  (bind _thislocation (Variables|Default|GetThisLocation))
  (return (Math|Vector|MakeVector (+ (.x _thislocation) (* (/ (- (.x (Variables|Default|GetRightRelativeLocation)) (.x (Variables|Default|GetLeftRelativeLocation))) 2.0) (* (- (Math|Random|RandomFloat) 0.5) 2.0))) (.y _thislocation) (.z _thislocation))))

(fn Init
  (Variables|Default|SetThisLocation (Transformation|GetActorLocation))
  (Variables|Default|SetLeftRelativeLocation (Variables|/Script/Engine.SceneComponent|GetRelativeLocation (Variables|Default|GetLeft)))
  (Variables|Default|SetRightRelativeLocation (Variables|/Script/Engine.SceneComponent|GetRelativeLocation (Variables|Default|GetRight)))
  (bind _returnvalue (Class|GameSingleton|GetGameSingleton))
  (bind _returnvalue_2 (Class|GameSingleton|GetInstance _returnvalue "/Script/MathDefence.MDGameNotifier"))
  (bind _asmdgame_notifier (Utilities|Casting|CastToMDGameNotifier _returnvalue_2))
  (Variables|Default|SetMainGameNotifier _asmdgame_notifier))

(fn CreateAttacker
  (bind _position (CallFunction|RandomPosition))
  (Game|SpawnActorfromClass "/Game/BluePrints/Game/BP_Attacker.BP_Attacker_C" (Math|Transform|MakeTransform _position "0, 0, 0" "0.400000,0.400000,0.400000") "Undefined" 0 0))

(fn HandleMainGameNotify
  (params (NotifyData :type Game%20Notify%20Data%20Structure))
  (switch Utilities|FlowControl|Switch|SwitchonMD_GAME_NOTIFY_ID (Utilities|Enum|ByteToEnumMD_GAME_NOTIFY_ID (Math|Conversions|ToByte(Integer) (.id NotifyData)))
    (:E_START_TO_CHECK_RESULT
      (bind _asinput_result_text (Utilities|Casting|CastToInputResultText (.data NotifyData)))
      (bind _returnvalue (Class|InputResultText|GetNumber _asinput_result_text))
      (Development|PrintString (Utilities|String|ToString(Integer) _returnvalue)))))